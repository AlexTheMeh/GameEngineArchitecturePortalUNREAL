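; Portal 1 of a linked pair: shows orange until Portal 2 exists, then a render-target material, and teleports overlapping actors to Portal 2.
; Players exit with yaw from Portal 2's render-target rotation, launched along its forward vector at stored speed.
; A briefly cleared GameMode flag limits re-teleporting, and collision is moved away and back to re-register overlaps.
; Tick yaws Portal1View using camera yaw and Portal 2's facing axis.
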(event `self.ReceiveTick`
  (params (DeltaSeconds :type "Float (single-precision)"))
  ;[1 1 1] Portal 1
  (set `self.Portal1ForwardVector` (0.0 0.0 0.0))
  (set `/Game/FirstPersonBP/Blueprints/FirstPersonCharacter.Portal1` (`SceneComponent.K2_GetComponentLocation` (`self.ArrowCentre`)) (`self.Cast To FPC`))
  (if (`KismetMathLibrary.EqualExactly_VectorVector` (`/Game/FirstPersonBP/Blueprints/FirstPersonCharacter.Portal2` (`self.Cast To FPC`)))
    (`PrimitiveComponent.SetMaterial` (`self.Plane`) 0 "/Game/Blueprint/Orange.Orange")
    (else
      (`PrimitiveComponent.SetMaterial` (`self.Plane`) 0 "/Game/Blueprint/Portal2_RT_Mat.Portal2_RT_Mat")
      (set `self.IsSecondPortalMade` true)
      (if (`/Game/FirstPersonBP/Blueprints/FirstPersonCharacter.NewlyCreatedPortal1` (`self.Cast To FPC`))
        (`self.ChangeOverlapPosition`))
      (`KismetSystemLibrary.Delay` DeltaSeconds)
      (`self.SetRenderTargetRotation`))))

(event `self.TeleportOnOverlap.OnComponentBeginOverlap`
  (params (OverlappedComponent :type "PrimitiveComponent Object Reference") (OtherActor :type "Actor Object Reference") (OtherComp :type "PrimitiveComponent Object Reference") (OtherBodyIndex :type Integer) (bFromSweep :type Boolean) (SweepResult :type "HitResult Structure (by ref)"))
  ;[1 1 1] Teleport Player + Set Player Rotation
  (bind _output_get (set `self.OverlappingActor` OtherActor))
  (if (`self.IsSecondPortalMade`)
    (bind _asfirst_person_character (cast `/Game/FirstPersonBP/Blueprints/FirstPersonCharacter` _output_get)
      (:`then`
        (set `self.IsPlayer` true)
        (set `self.Portal1ForwardVector` (`/Game/FirstPersonBP/Blueprints/FirstPersonCharacter.Portal1ForwardVector` _asfirst_person_character)))
      (:`CastFailed`
        (set `self.IsPlayer` false)))
    (bind _asfirst_person_game_mode (cast `/Game/FirstPersonBP/Blueprints/FirstPersonGameMode` (`GameplayStatics.GetGameMode`)))
    (if (`/Game/FirstPersonBP/Blueprints/FirstPersonGameMode.CanTeleport` _asfirst_person_game_mode)
      (set `/Game/FirstPersonBP/Blueprints/FirstPersonGameMode.CanTeleport` false _asfirst_person_game_mode)
      (`self.K2_SetActorLocation` _output_get (`/Game/FirstPersonBP/Blueprints/FirstPersonCharacter.Portal2` (`self.Cast To FPC`)) false true)
      (if (`self.IsPlayer`)
        (`self.SetPlayerRotation`)
        (`self.SetPlayerVelocity`))
      (`KismetSystemLibrary.Delay` 0.01)
      (bind _asfirst_person_game_mode_2 (cast `/Game/FirstPersonBP/Blueprints/FirstPersonGameMode` (`GameplayStatics.GetGameMode`)))
      (if (not (`/Game/FirstPersonBP/Blueprints/FirstPersonGameMode.CanTeleport` _asfirst_person_game_mode_2))
        (set `/Game/FirstPersonBP/Blueprints/FirstPersonGameMode.CanTeleport` true _asfirst_person_game_mode)))))

(event `self.ReceiveBeginPlay`
  ;[1 1 1] Set Collision Location Elsewhere for a micro second, and then teleport it back so that it registers overlap events!
  (set `self.Portal1Rot` (`SceneComponent.K2_GetComponentRotation` (`self.DefaultSceneRoot`)))
  (bind _asfirst_person_character (cast `/Game/FirstPersonBP/Blueprints/FirstPersonCharacter` (`GameplayStatics.GetPlayerCharacter` 0)))
  (set `self.Cast To FPC` _asfirst_person_character)
  (set `self.CollisionOriginalLocation` (`SceneComponent.K2_GetComponentLocation` (`self.TeleportOnOverlap`)) :!label _label)
  (`SceneComponent.K2_SetWorldLocation` (`self.TeleportOnOverlap`) (`self.CollisionRandomLocation`) false true)
  (`KismetSystemLibrary.Delay` 0.1)
  (`SceneComponent.K2_SetWorldLocation` (`self.TeleportOnOverlap`) (`self.CollisionOriginalLocation`) false true)
  (if (`self.FirstRun`)
    (set `self.FirstRun` false)
    (else
      (set `/Game/FirstPersonBP/Blueprints/FirstPersonCharacter.NewlyCreatedPortal1` false (`self.Cast To FPC`)))))

(event `ChangeOverlapPosition`
  ;[1 1 1] Set Collision Location Elsewhere for a micro second, and then teleport it back so that it registers overlap events!
  (goto _label))

(event `self.TeleportOnOverlap.OnComponentEndOverlap`
  (params (OverlappedComponent :type "PrimitiveComponent Object Reference") (OtherActor :type "Actor Object Reference") (OtherComp :type "PrimitiveComponent Object Reference") (OtherBodyIndex :type Integer))
  (cast `/Game/FirstPersonBP/Blueprints/FirstPersonCharacter` OtherActor)
  (`KismetSystemLibrary.Delay` 0.5)
  (`self.ResetMaxAcceleration`))

(fn `ResetMaxAcceleration`
  ;[1 1 1] Reset To Default Walk Speed, 600
  (set `CharacterMovementComponent.MaxAcceleration` 2048.0 (`Character.CharacterMovement` (`self.Cast To FPC`))))

(fn `SetLocationOnCall`
  (`/Game/FirstPersonBP/Blueprints/FirstPersonCharacter.DestroyPortal1` (`self.Cast To FPC`))
  (`|SpawnActorFromClass` "Portal1_C" (`KismetMathLibrary.MakeTransform` (`/Game/FirstPersonBP/Blueprints/FirstPersonCharacter.Portal1Location` (`self.Cast To FPC`)) (`self.Portal1Rot`)) "AdjustIfPossibleButDontSpawnIfColliding" "OverrideRootScale" null null) ; Spawn projectile
)

(fn `SetPlayerRotation`
  (bind _returnvalue (`GameplayStatics.GetPlayerController` 0))
  (bind (_portal2rendertargetrotation_roll _portal2rendertargetrotation_pitch _portal2rendertargetrotation_yaw) (`KismetMathLibrary.BreakRotator` (`/Game/FirstPersonBP/Blueprints/FirstPersonCharacter.Portal2RenderTargetRotation` (`self.Cast To FPC`))))
  ;[1 1 1] Get And Set Portal Location
  (set `self.Portal2Rot` (`/Game/FirstPersonBP/Blueprints/FirstPersonCharacter.Portal2Rotation` (`self.Cast To FPC`)))
  (set `self.Portal1Rot` (`SceneComponent.K2_GetComponentRotation` (`self.DefaultSceneRoot`)))
  (set `self.PlayerRot` (`self.K2_GetActorRotation` _returnvalue))
  (set `self.PlayerController` _returnvalue)
  (`Controller.SetControlRotation` (`self.PlayerController`) (`KismetMathLibrary.MakeRotator` 0.0 0.0 _portal2rendertargetrotation_yaw)))

(fn `SetPlayerVelocity`
  ;[0 0.166 0.7604] Get Velocity And Set Max Speed
  (set `CharacterMovementComponent.MaxAcceleration` 4096.0 (`Character.CharacterMovement` (`self.Cast To FPC`)))
  (if true
    (`/Game/FirstPersonBP/Blueprints/FirstPersonCharacter.StoreVelocity` (`self.Cast To FPC`))
    (set `self.Portal2ForwardVector` (`/Game/FirstPersonBP/Blueprints/FirstPersonCharacter.Portal2ForwardVector` (`self.Cast To FPC`)))
    (`self.SetVelocityAccordingToForwardVector`)))

(fn `SetRenderTargetRotation`
  (bind (_portal2forwardvector_x _portal2forwardvector_y) (`KismetMathLibrary.BreakVector` (`self.Portal2ForwardVector`)))
  (bind (_playerrot_roll _playerrot_pitch _playerrot_yaw) (`KismetMathLibrary.BreakRotator` (`self.PlayerRot`)))
  (bind (_playerrot_roll_2 _playerrot_pitch_2 _playerrot_yaw_2) (`KismetMathLibrary.BreakRotator` (`self.PlayerRot`)))
  (bind (_playerrot_roll_3 _playerrot_pitch_3 _playerrot_yaw_3) (`KismetMathLibrary.BreakRotator` (`self.PlayerRot`)))
  (bind (_playerrot_roll_4 _playerrot_pitch_4 _playerrot_yaw_4) (`KismetMathLibrary.BreakRotator` (`self.PlayerRot`)))
  (bind (_returnvalue_roll _returnvalue_pitch _returnvalue_yaw) (`KismetMathLibrary.BreakRotator` (`KismetMathLibrary.MakeRotator` 0.0 0.0 (- -90.0 _playerrot_yaw_4))))
  (bind (_returnvalue_roll_2 _returnvalue_pitch_2 _returnvalue_yaw_2) (`KismetMathLibrary.BreakRotator` (`KismetMathLibrary.MakeRotator` 0.0 0.0 (- 180.0 _playerrot_yaw))))
  (bind (_returnvalue_roll_3 _returnvalue_pitch_3 _returnvalue_yaw_3) (`KismetMathLibrary.BreakRotator` (`KismetMathLibrary.MakeRotator` 0.0 0.0 (- 90.0 _playerrot_yaw_3))))
  (set `self.PlayerRot` (`SceneComponent.K2_GetComponentRotation` (`PlayerCameraManager.TransformComponent` (`GameplayStatics.GetPlayerCameraManager` 0))))
  (set `self.Portal2ForwardVector` (`/Game/FirstPersonBP/Blueprints/FirstPersonCharacter.Portal2ForwardVector` (`self.Cast To FPC`)))
  ;[0 1 0.02183] Subtract Forward Vector Rotation from Current Player Rotation
  ;;[1 1 1] When Portal 2 Spawns at -X Axis
  (if (== _portal2forwardvector_x 1.0)
    (`SceneComponent.K2_SetRelativeRotation` (`self.Portal1View`) (`KismetMathLibrary.MakeRotator` 0.0 0.0 (* -1 _returnvalue_yaw_2)) false false)
    (else
      ;;[1 1 1] When Portal 2 Spawns at X Axis
      (if (== _portal2forwardvector_x -1.0)
        (`SceneComponent.K2_SetRelativeRotation` (`self.Portal1View`) (`KismetMathLibrary.MakeRotator` 0.0 0.0 _playerrot_yaw_2) false false)
        (else
          ;;[1 1 1] When Portal 2 Spawns at -Y Axis
          (if (== _portal2forwardvector_y 1.0)
            (`SceneComponent.K2_SetRelativeRotation` (`self.Portal1View`) (`KismetMathLibrary.MakeRotator` 0.0 0.0 (* -1 _returnvalue_yaw)) false false)
            (else
              ;;[1 1 1] When Portal 2 Spawns at  Y Axis
              (if (== _portal2forwardvector_y -1.0)
                (`SceneComponent.K2_SetRelativeRotation` (`self.Portal1View`) (`KismetMathLibrary.MakeRotator` 0.0 0.0 (* -1 _returnvalue_yaw_3)) false false)))))))))

(fn `SetVelocityAccordingToForwardVector`
  (`Character.LaunchCharacter` (`self.Cast To FPC`) (* (`self.Portal2ForwardVector`) (`KismetMathLibrary.VSize` (`/Game/FirstPersonBP/Blueprints/FirstPersonCharacter.PlayerVelocity` (`self.Cast To FPC`)))) true true))

(fn `UserConstructionScript`
  (`self.SetTickGroup` "TG_PostPhysics"))