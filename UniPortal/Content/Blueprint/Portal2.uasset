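; Second portal of a linked pair, teleporting any overlapping actor to Portal 1, with state shared through FirstPersonCharacter.
; Tick publishes its location, shows Portal 1's render-target material once that exists, and yaws Portal2View with the player camera.
; Players get axis-based yaw correction and relaunch along Portal 1's forward at current speed.
; A GameMode flag briefly gates re-teleporting; briefly moving the trigger away forces overlap events to register.
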(event `self.ReceiveTick`
  (params (DeltaSeconds :type "Float (single-precision)"))
  ;[1 1 1] Portal 2
  (set `self.Portal2ForwardVector` (`/Game/FirstPersonBP/Blueprints/FirstPersonCharacter.Portal2ForwardVector` (`self.Cast To FPC`)))
  (set `/Game/FirstPersonBP/Blueprints/FirstPersonCharacter.Portal2` (`SceneComponent.K2_GetComponentLocation` (`self.ArrowCentre`)) (`self.Cast To FPC`))
  (if (`KismetMathLibrary.EqualExactly_VectorVector` (`/Game/FirstPersonBP/Blueprints/FirstPersonCharacter.Portal1` (`self.Cast To FPC`)))
    (`PrimitiveComponent.SetMaterial` (`self.Plane`) 0 "/Game/Blueprint/Blue_Inst.Blue_Inst")
    (else
      (`PrimitiveComponent.SetMaterial` (`self.Plane`) 0 "/Game/Blueprint/Portal1_RT_Mat_Inst.Portal1_RT_Mat_Inst")
      (set `self.IsSecondPortalMade` true)
      (if (`/Game/FirstPersonBP/Blueprints/FirstPersonCharacter.NewlyCreatedPortal2` (`self.Cast To FPC`))
        (`self.RelocateTriggerBox`))
      (`KismetSystemLibrary.Delay` DeltaSeconds)
      (`self.SetRenderTargetRotation`)
      (bind _output_get (set `self.RenderTargetRotation` (`SceneComponent.K2_GetComponentRotation` (`self.Portal2View`))))
      (set `/Game/FirstPersonBP/Blueprints/FirstPersonCharacter.Portal2RenderTargetRotation` _output_get (`self.Cast To FPC`))
      (set `self.Portal1Rot` (`/Game/FirstPersonBP/Blueprints/FirstPersonCharacter.Portal1Rotation` (`self.Cast To FPC`))))))

(event `self.TeleportOnOverlap.OnComponentBeginOverlap`
  (params (OverlappedComponent :type "PrimitiveComponent Object Reference") (OtherActor :type "Actor Object Reference") (OtherComp :type "PrimitiveComponent Object Reference") (OtherBodyIndex :type Integer) (bFromSweep :type Boolean) (SweepResult :type "HitResult Structure (by ref)"))
  ;[0 1 0.2113] Teleport Player + Set The Players Rotation
  (if (`self.IsSecondPortalMade`)
    (bind _asfirst_person_character (cast `/Game/FirstPersonBP/Blueprints/FirstPersonCharacter` OtherActor)
      (:`then`
        (set `self.IsPlayer` true)
        (set `self.Portal2ForwardVector` (`/Game/FirstPersonBP/Blueprints/FirstPersonCharacter.Portal2ForwardVector` _asfirst_person_character)))
      (:`CastFailed`
        (set `self.IsPlayer` false)))
    (bind _asfirst_person_game_mode (cast `/Game/FirstPersonBP/Blueprints/FirstPersonGameMode` (`GameplayStatics.GetGameMode`)))
    (if (`/Game/FirstPersonBP/Blueprints/FirstPersonGameMode.CanTeleport` _asfirst_person_game_mode)
      (set `/Game/FirstPersonBP/Blueprints/FirstPersonGameMode.CanTeleport` false _asfirst_person_game_mode)
      (`self.K2_SetActorLocation` OtherActor (`/Game/FirstPersonBP/Blueprints/FirstPersonCharacter.Portal1` (`self.Cast To FPC`)) false true)
      (if (`self.IsPlayer`)
        (`self.SetPlayerRotation`)
        (`self.SetPlayerVelocity`))
      (`KismetSystemLibrary.Delay` 0.01)
      (bind _asfirst_person_game_mode_2 (cast `/Game/FirstPersonBP/Blueprints/FirstPersonGameMode` (`GameplayStatics.GetGameMode`)))
      (if (not (`/Game/FirstPersonBP/Blueprints/FirstPersonGameMode.CanTeleport` _asfirst_person_game_mode_2))
        (set `/Game/FirstPersonBP/Blueprints/FirstPersonGameMode.CanTeleport` true _asfirst_person_game_mode)))))

(event `self.ReceiveBeginPlay`
  ;[1 1 1] Set Collision Location Elsewhere for a micro second, and then teleport it back so that it registers overlap events!
  (set `self.Portal2Rot` (`SceneComponent.K2_GetComponentRotation` (`self.DefaultSceneRoot`)))
  (bind _asfirst_person_character (cast `/Game/FirstPersonBP/Blueprints/FirstPersonCharacter` (`GameplayStatics.GetPlayerCharacter` 0)))
  (set `self.Cast To FPC` _asfirst_person_character)
  (set `self.CollisionOriginalLocation` (`SceneComponent.K2_GetComponentLocation` (`self.TeleportOnOverlap`)) :!label _label)
  (`SceneComponent.K2_SetWorldLocation` (`self.TeleportOnOverlap`) (`self.CollisionRandomLocation`) false true)
  (`KismetSystemLibrary.Delay` 0.1)
  (`SceneComponent.K2_SetWorldLocation` (`self.TeleportOnOverlap`) (`self.CollisionOriginalLocation`) false true)
  (if (`self.FirstRun`)
    (set `self.FirstRun` false))
  (set `/Game/FirstPersonBP/Blueprints/FirstPersonCharacter.NewlyCreatedPortal2` false (`self.Cast To FPC`)))

(event `RelocateTriggerBox`
  ;[1 1 1] Set Collision Location Elsewhere for a micro second, and then teleport it back so that it registers overlap events!
  (goto _label))

(event `self.TeleportOnOverlap.OnComponentEndOverlap`
  (params (OverlappedComponent :type "PrimitiveComponent Object Reference") (OtherActor :type "Actor Object Reference") (OtherComp :type "PrimitiveComponent Object Reference") (OtherBodyIndex :type Integer))
  (`KismetSystemLibrary.Delay` 0.5)
  (`self.ResetMaxAcceleration`))

(fn `RenderTargetLocation`
  (`SceneComponent.K2_SetRelativeLocation` (`self.Portal2View`) (- (`SceneComponent.K2_GetComponentLocation` (`Actor.RootComponent` (`self.Cast To FPC`))) (`/Game/FirstPersonBP/Blueprints/FirstPersonCharacter.Portal1Location` (`self.Cast To FPC`))) false false))

(fn `ResetMaxAcceleration`
  ;[0 1 0.8423] Reset Acceleration
  (set `CharacterMovementComponent.MaxAcceleration` 2048.0 (`Character.CharacterMovement` (`self.Cast To FPC`))))

(fn `SetLocationOnCall`
  (`/Game/FirstPersonBP/Blueprints/FirstPersonCharacter.DestroyPortal2` (`self.Cast To FPC`))
  (`|SpawnActorFromClass` "Portal2_C" (`KismetMathLibrary.MakeTransform` (`/Game/FirstPersonBP/Blueprints/FirstPersonCharacter.Portal2Location` (`self.Cast To FPC`)) (`self.Portal2Rot`)) "AdjustIfPossibleButDontSpawnIfColliding" "OverrideRootScale" null null) ; Spawn projectile
)

(fn `SetPlayerRotation`
  (bind _returnvalue (`GameplayStatics.GetPlayerController` 0))
  (bind (_playerrot_roll _playerrot_pitch _playerrot_yaw) (`KismetMathLibrary.BreakRotator` (`self.PlayerRot`)))
  (bind (_playerrot_roll_2 _playerrot_pitch_2 _playerrot_yaw_2) (`KismetMathLibrary.BreakRotator` (`self.PlayerRot`)))
  (bind (_playerrot_roll_3 _playerrot_pitch_3) (`KismetMathLibrary.BreakRotator` (`self.PlayerRot`)))
  (bind (_portal1rot_roll _portal1rot_pitch _portal1rot_yaw) (`KismetMathLibrary.BreakRotator` (`self.Portal1Rot`)))
  (bind (_playerrot_roll_4 _playerrot_pitch_4 _playerrot_yaw_3) (`KismetMathLibrary.BreakRotator` (`self.PlayerRot`)))
  (bind (_playerrot_roll_5 _playerrot_pitch_5 _playerrot_yaw_4) (`KismetMathLibrary.BreakRotator` (`self.PlayerRot`)))
  (bind (_portal1rot_roll_2 _portal1rot_pitch_2 _portal1rot_yaw_2) (`KismetMathLibrary.BreakRotator` (`self.Portal1Rot`)))
  (bind (_playerrot_roll_6 _playerrot_pitch_6 _playerrot_yaw_5) (`KismetMathLibrary.BreakRotator` (`self.PlayerRot`)))
  (bind (_playerrot_roll_7 _playerrot_pitch_7 _playerrot_yaw_6) (`KismetMathLibrary.BreakRotator` (`self.PlayerRot`)))
  (bind (_portal1rot_roll_3 _portal1rot_pitch_3 _portal1rot_yaw_3) (`KismetMathLibrary.BreakRotator` (`self.Portal1Rot`)))
  (bind (_playerrot_roll_8 _playerrot_pitch_8 _playerrot_yaw_7) (`KismetMathLibrary.BreakRotator` (`self.PlayerRot`)))
  (bind (_playerrot_roll_9 _playerrot_pitch_9 _playerrot_yaw_8) (`KismetMathLibrary.BreakRotator` (`self.PlayerRot`)))
  (bind (_portal1rot_roll_4 _portal1rot_pitch_4 _portal1rot_yaw_4) (`KismetMathLibrary.BreakRotator` (`self.Portal1Rot`)))
  (bind (_playerrot_roll_10 _playerrot_pitch_10 _playerrot_yaw_9) (`KismetMathLibrary.BreakRotator` (`self.PlayerRot`)))
  (bind (_portal1rot_roll_5 _portal1rot_pitch_5 _portal1rot_yaw_5) (`KismetMathLibrary.BreakRotator` (`self.Portal1Rot`)))
  ;[1 1 1] Get And Set Portal Location
  (set `self.Portal1Rot` (`/Game/FirstPersonBP/Blueprints/FirstPersonCharacter.Portal1Rotation` (`self.Cast To FPC`)))
  (set `self.Portal2Rot` (`SceneComponent.K2_GetComponentRotation` (`self.DefaultSceneRoot`)))
  (set `self.PlayerRot` (`self.K2_GetActorRotation` _returnvalue))
  (set `self.PlayerController` _returnvalue)
  ;[1 1 1] Rotate Player 180 Deg if Portal Is Placed On The Same Axis
  (if (== (`self.Portal1Rot`) (`self.Portal2Rot`) :`ErrorTolerance` 1.0)
    (`Controller.SetControlRotation` (`self.PlayerController`) (`KismetMathLibrary.MakeRotator` _playerrot_roll _playerrot_pitch (+ _playerrot_yaw 180.0)))
    (else
      ;[1 1 1] If Portal 2 Is Opposite of Portal 1, Don't Do Anything, Because Forward Axis Will Remain Same
      (if (not (or (== (* (`self.Portal2Rot`) -1) (`self.Portal1Rot`) :`ErrorTolerance` 1.0) (and (== (`self.Portal2Rot`) (struct :`Yaw` 180.0) :`ErrorTolerance` 1.0) (== (`self.Portal1Rot`) (struct) :`ErrorTolerance` 1.0)) (and (== (`self.Portal2Rot`) (struct) :`ErrorTolerance` 1.0) (== (`self.Portal1Rot`) (struct :`Yaw` 180.0) :`ErrorTolerance` 1.0))))
        ;[1 1 1] If Portal 2 Axis = X, Rotate Player According To Rotation Of Portal 1
        (if (== (`self.Portal2Rot`) (struct :`Yaw` -180.0) :`ErrorTolerance` 1.0)
          (if (`KismetMathLibrary.NearlyEqual_FloatFloat` _portal1rot_yaw 90.0 1.0)
            (`Controller.SetControlRotation` (`self.PlayerController`) (`KismetMathLibrary.MakeRotator` _playerrot_roll_4 _playerrot_pitch_4 (+ _playerrot_yaw_3 90.0)))
            (else
              (`Controller.SetControlRotation` (`self.PlayerController`) (`KismetMathLibrary.MakeRotator` _playerrot_roll_2 _playerrot_pitch_2 (- _playerrot_yaw_2 90.0)))))
          (else
            ;[1 1 1] If Portal 2 Axis = -X, Rotate Player According To Rotation Of Portal 1
            (if (== (`self.Portal2Rot`) (struct) :`ErrorTolerance` 1.0)
              (if (`KismetMathLibrary.NearlyEqual_FloatFloat` _portal1rot_yaw_2 -90.0 1.0)
                (`Controller.SetControlRotation` (`self.PlayerController`) (`KismetMathLibrary.MakeRotator` _playerrot_roll_5 _playerrot_pitch_5 (+ _playerrot_yaw_4 90.0)))
                (else
                  (`Controller.SetControlRotation` (`self.PlayerController`) (`KismetMathLibrary.MakeRotator` _playerrot_roll_6 _playerrot_pitch_6 (- _playerrot_yaw_5 90.0)))))
              (else
                ;[1 1 1] If Portal 2 Axis = Y, Rotate Player According To Rotation Of Portal 1
                (if (== (`self.Portal2Rot`) (struct :`Yaw` -90.0) :`ErrorTolerance` 1.0)
                  (if (`KismetMathLibrary.NearlyEqual_FloatFloat` _portal1rot_yaw_3 0.0 1.0)
                    (`Controller.SetControlRotation` (`self.PlayerController`) (`KismetMathLibrary.MakeRotator` _playerrot_roll_7 _playerrot_pitch_7 (+ _playerrot_yaw_6 -90.0)))
                    (else
                      (`Controller.SetControlRotation` (`self.PlayerController`) (`KismetMathLibrary.MakeRotator` _playerrot_roll_8 _playerrot_pitch_8 (+ _playerrot_yaw_7 90.0)))))
                  (else
                    ;[1 1 1] If Portal 2 Axis = -Y, Rotate Player According To Rotation Of Portal 1
                    (if (== (`self.Portal2Rot`) (struct :`Yaw` 90.0) :`ErrorTolerance` 1.0)
                      (if (`KismetMathLibrary.NearlyEqual_FloatFloat` _portal1rot_yaw_4 0.0 1.0)
                        (`Controller.SetControlRotation` (`self.PlayerController`) (`KismetMathLibrary.MakeRotator` _playerrot_roll_9 _playerrot_pitch_9 (+ _playerrot_yaw_8 90.0)))
                        (else
                          (`Controller.SetControlRotation` (`self.PlayerController`) (`KismetMathLibrary.MakeRotator` _playerrot_roll_10 _playerrot_pitch_10 (+ _playerrot_yaw_9 -90.0)))))
                      (else
                        ;[1 1 1] If Portal 2 Axis = Z, Rotate Player According To Rotation Of Portal 1
                        (if (== (`self.Portal2Rot`) (struct :`Pitch` 90.0) :`ErrorTolerance` 1.0)
                          (`Controller.SetControlRotation` (`self.PlayerController`) (`KismetMathLibrary.MakeRotator` _playerrot_roll_3 _playerrot_pitch_3 _portal1rot_yaw_5)))))))))))))))

(fn `SetPlayerVelocity`
  ;[1 0.526 0] Get Velocity And Set Max Speed
  (set `CharacterMovementComponent.MaxAcceleration` 4096.0 (`Character.CharacterMovement` (`self.Cast To FPC`)))
  (if true
    (`/Game/FirstPersonBP/Blueprints/FirstPersonCharacter.StoreVelocity` (`self.Cast To FPC`))
    (set `self.Portal1ForwardVector` (`/Game/FirstPersonBP/Blueprints/FirstPersonCharacter.Portal1ForwardVector` (`self.Cast To FPC`)))
    (`self.SetVelocityAccordingToForwardVector`)))

(fn `SetRenderTargetRotation`
  (locals (NewLocalVar_0 :type "Vector Structure" :default (0.0 0.0 0.0)))
  (bind (_portal1forwardvector_x _portal1forwardvector_y) (`KismetMathLibrary.BreakVector` (`self.Portal1ForwardVector`)))
  (bind (_playerrot_roll _playerrot_pitch _playerrot_yaw) (`KismetMathLibrary.BreakRotator` (`self.PlayerRot`)))
  (bind (_playerrot_roll_2 _playerrot_pitch_2 _playerrot_yaw_2) (`KismetMathLibrary.BreakRotator` (`self.PlayerRot`)))
  (bind (_playerrot_roll_3 _playerrot_pitch_3 _playerrot_yaw_3) (`KismetMathLibrary.BreakRotator` (`self.PlayerRot`)))
  (bind (_playerrot_roll_4 _playerrot_pitch_4 _playerrot_yaw_4) (`KismetMathLibrary.BreakRotator` (`self.PlayerRot`)))
  (bind (_returnvalue_roll _returnvalue_pitch _returnvalue_yaw) (`KismetMathLibrary.BreakRotator` (`KismetMathLibrary.MakeRotator` 0.0 0.0 (- 180.0 _playerrot_yaw))))
  (bind (_returnvalue_roll_2 _returnvalue_pitch_2 _returnvalue_yaw_2) (`KismetMathLibrary.BreakRotator` (`KismetMathLibrary.MakeRotator` 0.0 0.0 (- -90.0 _playerrot_yaw_4))))
  (bind (_returnvalue_roll_3 _returnvalue_pitch_3 _returnvalue_yaw_3) (`KismetMathLibrary.BreakRotator` (`KismetMathLibrary.MakeRotator` 0.0 0.0 (- 90.0 _playerrot_yaw_3))))
  (set `self.PlayerRot` (`SceneComponent.K2_GetComponentRotation` (`PlayerCameraManager.TransformComponent` (`GameplayStatics.GetPlayerCameraManager` 0))))
  (set `self.Portal1ForwardVector` (`/Game/FirstPersonBP/Blueprints/FirstPersonCharacter.Portal1ForwardVector` (`self.Cast To FPC`)))
  ;[0 1 0.02183] Subtract Forward Vector Rotation from Current Player Rotation
  ;;[1 1 1] When Portal 2 Spawns at -X Axis
  (if (== _portal1forwardvector_x 1.0)
    (`SceneComponent.K2_SetRelativeRotation` (`self.Portal2View`) (`KismetMathLibrary.MakeRotator` 0.0 0.0 (* -1 _returnvalue_yaw)) false false)
    (else
      ;;[1 1 1] When Portal 2 Spawns at X Axis
      (if (== _portal1forwardvector_x -1.0)
        (`SceneComponent.K2_SetRelativeRotation` (`self.Portal2View`) (`KismetMathLibrary.MakeRotator` 0.0 0.0 _playerrot_yaw_2) false false)
        (else
          ;;[1 1 1] When Portal 2 Spawns at -Y Axis
          (if (== _portal1forwardvector_y 1.0)
            (`SceneComponent.K2_SetRelativeRotation` (`self.Portal2View`) (`KismetMathLibrary.MakeRotator` 0.0 0.0 (* -1 _returnvalue_yaw_2)) false false)
            (else
              ;;[1 1 1] When Portal 2 Spawns at  Y Axis
              (if (== _portal1forwardvector_y -1.0)
                (`SceneComponent.K2_SetRelativeRotation` (`self.Portal2View`) (`KismetMathLibrary.MakeRotator` 0.0 0.0 (* -1 _returnvalue_yaw_3)) false false)))))))))

(fn `SetVariables`)

(fn `SetVelocityAccordingToForwardVector`
  (`Character.LaunchCharacter` (`self.Cast To FPC`) (* (`self.Portal1ForwardVector`) (`KismetMathLibrary.VSize` (`self.GetVelocity` (`self.Cast To FPC`)))) true true))

(fn `UserConstructionScript`
  (`self.SetTickGroup` "TG_PostPhysics"))